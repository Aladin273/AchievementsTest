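; BP_ATGameHUD is the game HUD that swaps the on-screen widget to match the game mode's match state.
; On BeginPlay it binds to the ATGameModeBase state-changed event.
; Each change removes the current widget, then creates and adds the one selected for the new state: gameplay overlay, pause or game over.
; WaitingForStart has no widget class assigned.
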(event Custom|Game%20Mode%20State
  (params (MatchState :type EATGameModeState%20Enum :default "WaitingForStart"))
  (Utilities|FlowControl|Sequence
    (:then_0
      (Utilities|IsValid (Variables|Default|GetCurrent%20Widget)
        (:Is%20Valid
          (Widget|RemovefromParent (Variables|Default|GetCurrent%20Widget)))))
    (:then_1
      (bind _returnvalue (UserInterface|CreateWidget (Utilities|Select :Index MatchState :WaitingForStart 0 :InProgress "/Game/UI/WBP_GameOverlay.WBP_GameOverlay_C" :Pause "/Game/UI/WBP_GamePause.WBP_GamePause_C" :GameOver "/Game/UI/WBP_GameOver.WBP_GameOver_C")))
      (UserInterface|Viewport|AddtoViewport _returnvalue 0)
      (Variables|Default|SetCurrent%20Widget _returnvalue))))

(event EventBeginPlay
  (bind _asatgame_mode_base (Utilities|Casting|CastToATGameModeBase (Game|GetGameMode)))
  (EventDispatchers|BindEventtoOnGameModeStateChanged _asatgame_mode_base (delegate Custom|Game%20Mode%20State)))

(fn ConstructionScript)