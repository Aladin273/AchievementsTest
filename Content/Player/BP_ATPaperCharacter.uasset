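; BP_ATPaperCharacter is the player character that reports gameplay actions to the achievements subsystem as progress.
; It reports game start, jumps and trigger box overlaps as they happen, while overlapping a game-over box calls GameOver on the game mode.
; Tick accumulates horizontal distance from movement velocity, and a looping one-second timer is set up to report it as truncated Walk progress and reset it.
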(event Custom|Walk%20Timer
  (Class|ATAchievementsSubsystem|AddAchievementProgress (Subsystems|GetATAchievementsSubsystem) "Walk" (Math|Float|Truncate (Variables|Default|GetDistanceTraveled)))
  (Variables|Default|SetDistanceTraveled 0.0))

(event EventBeginPlay
  (Utilities|Time|SetTimerbyFunctionName 0 "Walk TImer" 1.0 true)
  (Class|ATAchievementsSubsystem|AddAchievementProgress (Subsystems|GetATAchievementsSubsystem) "Start" 1))

(event Collision|EventActorBeginOverlap
  (params (OtherActor :type Actor%20Object%20Reference))
  (Utilities|Casting|CastToBP_ATTriggerBox OtherActor
    (:then
      (Class|ATAchievementsSubsystem|AddAchievementProgress (Subsystems|GetATAchievementsSubsystem) "Trigger" 1))
    (:CastFailed
      (Utilities|Casting|CastToBP_ATGameOverBox OtherActor)
      (bind _asatgame_mode_base (Utilities|Casting|CastToATGameModeBase (Game|GetGameMode)))
      (Class|ATGameModeBase|GameOver _asatgame_mode_base))))

(event EventTick
  (params (DeltaSeconds :type Float%20%28single-precision%29))
  (bind _charactermovement (Variables|Character|GetCharacterMovement))
  (bind _velocity (Variables|/Script/Engine.MovementComponent|GetVelocity _charactermovement))
  (Variables|Default|SetDistanceTraveled (+ (Math|Vector|VectorLength (* DeltaSeconds (Math|Vector|MakeVector (.x _velocity) (.y _velocity) 0.0))) (Variables|Default|GetDistanceTraveled))))

(event EventOnJumped
  (Class|ATAchievementsSubsystem|AddAchievementProgress (Subsystems|GetATAchievementsSubsystem) "Jump" 1))

(fn ConstructionScript)